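; BP_TTT_Field is a single clickable board field for what appears to be a tic-tac-toe game.
; Cursor hover swaps in a highlight material and restores the original on exit, but only while the field is unclaimed.
; A click records the game mode's current player, reports the FieldId to BP_TTT_GameMode, then applies that player's material.
; The click handler itself does not check whether the field is already claimed.
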(event `self.ReceiveBeginPlay`
  (add `self.OnBeginCursorOver` (delegate `OnHoverStart`))
  (add `self.OnEndCursorOver` (delegate `OnHoverEnd`))
  (add `self.OnClicked` (delegate `OnClickedEvent`))
  (set `self.OriginalMaterial` (`PrimitiveComponent.GetMaterial` (`self.StaticMeshComponent`) 0))
  (bind _asbp_ttt_game_mode (cast `/Game/Project01/Blueprints/BP_TTT_GameMode` (`GameplayStatics.GetGameMode`)))
  (set `self.TTTGameMode` _asbp_ttt_game_mode))

(event `OnHoverEnd` :!signature `self.OnEndCursorOver`
  (params (TouchedActor :type "Actor Object Reference"))
  (if (not (`self.WasClicked`))
    (`PrimitiveComponent.SetMaterial` (`self.StaticMeshComponent`) 0 (`self.OriginalMaterial`))))

(event `OnClickedEvent` :!signature `self.OnClicked`
  (params (TouchedActor :type "Actor Object Reference") (ButtonPressed :type "Key Structure" :default "None"))
  (set `self.ClickedBy` (`/Game/Project01/Blueprints/BP_TTT_GameMode.CurrentPlayer` (`self.TTTGameMode`)))
  (`/Game/Project01/Blueprints/BP_TTT_GameMode.OnPlayerClicked` (`self.TTTGameMode`) (`self.FieldId`))
  (`PrimitiveComponent.SetMaterial` (`self.StaticMeshComponent`) 0 (`|GetArrayItem` (`self.ClickedMaterial`) (`self.ClickedBy`))))

(event `OnHoverStart` :!signature `self.OnBeginCursorOver`
  (params (TouchedActor :type "Actor Object Reference"))
  (if (not (`self.WasClicked`))
    (`PrimitiveComponent.SetMaterial` (`self.StaticMeshComponent`) 0 (`self.HoverMaterial`))))

(fn `UserConstructionScript`)

(fn `WasClicked`
  (returns (WasClicked :type Boolean))
  (return (> (`self.ClickedBy`) -1)))